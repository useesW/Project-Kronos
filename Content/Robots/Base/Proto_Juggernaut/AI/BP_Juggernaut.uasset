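; Juggernaut enemy robot that tracks the player and fires projectiles from both guns while it has line of sight.
; Tick traces to the player, aims a Control Rig target, slowly yaws the body and shoots on a fire-rate timer.
; Projectile overlaps on the armor collider deplete armor until the plate detaches with physics.
; The next hit ragdolls the robot with a backward impulse and calls Die on its AI_Guard controller.
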(event OnPreInitializeDelegate(ControlRig)
  (params (Component :type Control%20Rig%20Component%20Object%20Reference))
  (Class|ControlRigComponent|AddMappedCompleteSkeletalMesh Component (Variables|Character|GetMesh)))

(event OnComponentBeginOverlap(ArmorCol)
  (params (OverlappedComponent :type Primitive%20Component%20Object%20Reference) (OtherActor :type Actor%20Object%20Reference) (OtherComp :type Primitive%20Component%20Object%20Reference) (OtherBodyIndex :type Integer) (bFromSweep :type Boolean) (SweepResult :type Hit%20Result%20Structure%20%28by%20ref%29))
  (bind _mesh (Variables|Character|GetMesh))
  (bind _armorplate (Variables|Default|GetArmorPlate))
  ;[1 1 1] Handle AI Death On Projectile Impact
  ;;[1 1 1] Don't Re-Die
  (if (not (Variables|Default|GetIsDead))
    (Utilities|Casting|CastToBP_Master_Projectile OtherActor)
    ;;[1 1 1] If Armor Plate Has Not Been Shot Off
    (if (Variables|Default|GetIsWeak)
      ;;[1 1 1] Enter Ragdoll & Stop AI
      (Physics|SetSimulatePhysics _mesh true)
      ;;;[1 1 1] Add Backwards Impulse For Effect
      (Physics|AddImpulse _mesh (* (Class|KismetMathLibrary|VectorForward) (Math|Conversions|ToVector(Float) -2e+03)) "Spine_01" true)
      (Variables|Default|SetIsDead true)
      ;;;[1 1 1] Stop AI
      (bind _asai_guard (Utilities|Casting|CastToAI_Guard (AI|GetAIController self))
        (:then
          (Default|Die _asai_guard))
        (:CastFailed
          (Development|PrintString "Done Goofed")))
      (Collision|SetCollisionEnabled (Variables|Collision|GetCapsuleComponent) "NoCollision")
      (else
        ;;[1 1 1] Control The Ammount Of Shots It Takes To Break Armor
        (if (<= (Variables|Default|GetArmor%20Health) 0.0)
          ;;[1 1 1] Break Armor Plate And Enter Weak State
          (Components|SkinnedMesh|SetLeaderPoseComponent _armorplate 0 false false)
          (Utilities|FlowControl|Delay 0.1)
          (Physics|SetSimulatePhysics _armorplate true)
          (Physics|AddImpulse _armorplate "0.000000,0.000000,10000.000000" "None" true)
          (Variables|Default|SetIsWeak true)
          (else
            (Variables|Default|SetArmor%20Health (- (Variables|Default|GetArmor%20Health) 1e+01))))))))

(event Custom|Shoot
  (bind _projectilespawnlocations (Variables|Default|GetProjectileSpawnLocations))
  (bind _mesh (Variables|Character|GetMesh))
  (bind _mesh_2 (Variables|Character|GetMesh))
  (bind _projectilespawnlocations_2 (Variables|Default|GetProjectileSpawnLocations))
  (bind _returnvalue (Transformation|GetSocketTransform _mesh "Gun_R" "RTS_World"))
  (bind _returnvalue_2 (Transformation|GetSocketTransform _mesh_2 "Gun_L" "RTS_World"))
  (bind _output (Utilities|Array|Get(acopy) _projectilespawnlocations 1))
  (bind _output_2 (Utilities|Array|Get(acopy) _projectilespawnlocations_2))
  (bind _location (Math|Transform|BreakTransform _returnvalue))
  (bind _returnvalue_3 (Math|Transform|TransformDirection _returnvalue _output))
  (bind _location_2 (Math|Transform|BreakTransform _returnvalue_2))
  (bind _returnvalue_4 (Math|Transform|TransformDirection _returnvalue_2 _output_2))
  (bind _returnvalue_5 (+ _location_2 _returnvalue_4))
  (bind _returnvalue_6 (+ _location _returnvalue_3))
  ;[1 1 1] Shoot
  (Variables|Default|SetTimeSinceLastShot (Utilities|Time|GetTimeSeconds))
  (Game|SpawnActorfromClass "/Game/FirstPerson/Blueprints/BP_Master_Projectile.BP_Master_Projectile_C" (Math|Transform|MakeTransform _returnvalue_5 (Math|Rotator|FindLookatRotation _returnvalue_5 (+ (Transformation|GetActorLocation (Game|GetPlayerCharacter 0)) "0.000000,0.000000,50.000000"))) "Undefined" 0 0)
  ;[1 1 1] Play Audio
  (Audio|PlaySoundatLocation "/Game/FPWeapon/Audio/EnemyShoot.EnemyShoot" _returnvalue_5 "0, 0, 0" 1.0 1.0 0.0 0 0 0 0) ; Play firing sound
  (Game|SpawnActorfromClass "/Game/FirstPerson/Blueprints/BP_Master_Projectile.BP_Master_Projectile_C" (Math|Transform|MakeTransform _returnvalue_6 (Math|Rotator|FindLookatRotation _returnvalue_6 (+ (Transformation|GetActorLocation (Game|GetPlayerCharacter 0)) "0.000000,0.000000,50.000000"))) "Undefined" 0 0)
  (Audio|PlaySoundatLocation "/Game/FPWeapon/Audio/EnemyShoot.EnemyShoot" _returnvalue_6 "0, 0, 0" 1.0 1.0 0.0 0 0 0 0) ; Play firing sound
)

(event Custom|HandleRotation
  ;[1 1 1] Set Control Rig Target Position So The AI Will Look/Aim Towards The Player
  (Class|ControlRigComponent|SetControlPosition (Variables|Default|GetControlRig) "CTR_Target" (Math|Vector|RotateVector (+ (Math|Vector|RotateVectorAroundAxis (- (Transformation|GetActorLocation (Game|GetPlayerCharacter 0)) (Transformation|GetActorLocation)) 9e+01 "0.000000,0.000000,1.000000") "0.000000,0.000000,100.000000") (Class|KismetMathLibrary|NegateRotator (Transformation|GetActorRotation))) "ActorSpace")
  ;[1 1 1] Slowly rotate the robot to face the player
  (Transformation|SetActorRotation (Math|Rotator|MakeRotator 0.0 0.0 (.Yaw (Math|Rotator|BreakRotator (Math|Rotator|Lerp(Rotator) (Transformation|GetActorRotation) (Math|Rotator|FindLookatRotation (Transformation|GetActorLocation) (Transformation|GetActorLocation (Game|GetPlayerCharacter 0))) (* (Utilities|Time|GetWorldDeltaSeconds) 1.0) true))))))

(event Custom|Show%20Projectile%20Spawn%20Location
  (params (isShown :type Boolean))
  (bind _mesh (Variables|Character|GetMesh))
  (bind _mesh_2 (Variables|Character|GetMesh))
  (bind _returnvalue (Transformation|GetSocketTransform _mesh_2 "Gun_R" "RTS_World"))
  (bind _returnvalue_2 (Transformation|GetSocketTransform _mesh "Gun_L" "RTS_World"))
  ;[1 1 1] Visualize Projectile Spawn Position
  (if isShown
    (Rendering|Debug|DrawDebugSphere (+ (.Location (Math|Transform|BreakTransform _returnvalue_2)) (Math|Transform|TransformDirection _returnvalue_2 (Utilities|Array|Get(acopy) (Variables|Default|GetProjectileSpawnLocations)))) 1e+01 12 "(R=0.000000,G=1.000000,B=0.578555,A=1.000000)" 0.0 0.5)
    (Rendering|Debug|DrawDebugSphere (+ (.Location (Math|Transform|BreakTransform _returnvalue)) (Math|Transform|TransformDirection _returnvalue (Utilities|Array|Get(acopy) (Variables|Default|GetProjectileSpawnLocations) 1))) 1e+01 12 "(R=0.000000,G=1.000000,B=0.578555,A=1.000000)" 0.0 0.5)))

(event EventBeginPlay)

(event Collision|EventActorBeginOverlap
  (params (OtherActor :type Actor%20Object%20Reference)))

(event EventTick
  (params (DeltaSeconds :type Float%20%28single-precision%29))
  (if (not (Variables|Default|GetIsDead))
    ;[1 1 1] If The Player is in line of sight, Look & Shoot
    (bind _outhit (Collision|LineTraceByChannel (Transformation|GetActorLocation) (+ (Transformation|GetActorLocation (Game|GetPlayerCharacter 0)) "0.000000,0.000000,50.000000") "TraceTypeQuery2" false 0 "None"))
    (Utilities|Casting|CastToBP_FirstPersonCharacter (.HitActor (Collision|BreakHitResult _outhit)))
    (CallFunction|HandleRotation)
    (CallFunction|ShowProjectileSpawnLocation false)
    (if (>= (- (Utilities|Time|GetTimeSeconds) (Variables|Default|GetTimeSinceLastShot)) (Variables|Default|GetFireRate))
      (CallFunction|Shoot))))

(fn ConstructionScript)