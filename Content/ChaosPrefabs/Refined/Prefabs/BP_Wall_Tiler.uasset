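; BP_Wall_Tiler is a construction-script actor that assembles a row of wall pieces from an ordered array of actor classes, TileOrder.
; For each valid class it adds a child actor component at the running TileOffset.
; It then steps the offset along negative local Y by a Y value read from that class's defaults, so pieces of differing size chain in sequence.
; The event graph is empty.
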(event EventBeginPlay)

(event Collision|EventActorBeginOverlap
  (params (OtherActor :type Actor%20Object%20Reference)))

(event EventTick
  (params (DeltaSeconds :type Float%20%28single-precision%29)))

(fn ConstructionScript
  (Variables|Default|SetTileOffset "0, 0, 0")
  (for _array_element (Variables|WallGeneration|GetTileOrder)
    (if (Utilities|IsValidClass _array_element)
      (bind _returnvalue (AddComponent|AddChildActorComponent false (Math|Transform|MakeTransform (Variables|Default|GetTileOffset))))
      (ChildActorComponent|SetChildActorClass _returnvalue _array_element)
      (Variables|Default|SetTileOffset (Math|Vector|MakeVector 0.0 (- (.Y (Math|Vector|BreakVector (Variables|Default|GetTileOffset))) (.Y (Class|KismetMathLibrary|BreakVector3f (Utilities|GetClassDefaults _array_element)))) 0.0)))))