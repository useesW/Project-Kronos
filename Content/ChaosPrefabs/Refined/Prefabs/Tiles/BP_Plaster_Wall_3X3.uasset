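; Destructible 3X3 plaster wall tile prefab built from Chaos Geometry Collections: front and back plaster sheets plus two studs.
; The construction script picks random collections for each pair from geometry arrays, using a retry loop intended to avoid duplicates within a pair.
; It then registers child-actor anchor fields as initialization fields, with all four edges on the sheets and only top and bottom on the studs.
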(event EventBeginPlay
  (|CallParentFunction) ; This node is disabled and will not be called.\nDrag off pins to build functionality.
)

(event Collision|EventActorBeginOverlap
  (params (OtherActor :type Actor%20Object%20Reference))
  (|CallParentFunction OtherActor) ; This node is disabled and will not be called.\nDrag off pins to build functionality.
)

(event EventTick
  (params (DeltaSeconds :type Float%20%28single-precision%29))
  (|CallParentFunction DeltaSeconds) ; This node is disabled and will not be called.\nDrag off pins to build functionality.
)

(fn ConstructionScript
  (CallFunction|InitializePlasterSheets)
  (CallFunction|InitializeStuds)
  (CallFunction|SetAnchors))

(fn InitializePlasterSheets
  (bind _plastergeometry (Variables|Initialization|GetPlasterGeometry))
  (bind _returnvalue (Utilities|Array|Length _plastergeometry))
  (bind _returnvalue_2 (- _returnvalue 1))
  (bind _returnvalue_3 (Math|Random|RandomInteger _returnvalue_2))
  ;[1 1 1] Assign The Front Plaster Sheet With A Random GC From The Array
  (bind _output_get (Variables|Initialization|SetSelectionIndex (Math|Random|RandomInteger (- (Utilities|Array|Length (Variables|Initialization|GetPlasterGeometry)) 1))))
  (Class|GeometryCollectionComponent|SetRestCollection (Variables|Default|GetGC_Plaster_Front) (Utilities|Array|Get(acopy) (Variables|Initialization|GetPlasterGeometry) _output_get))
  ;[1 1 1] Select Another GC, But Do Not Use Previous One (FailSafe = Unless Only One Exist In Array)
  (Utilities|FlowControl|DoOnce false :!label _label
    (:Completed
      (if (and (!= _returnvalue 1) (== (Variables|Initialization|GetSelectionIndex) _returnvalue_3))
        (goto _label Reset)
        (else
          ;[1 1 1] Assign The Random GC To The Back Plaster Sheet
          (bind _output_get_2 (Variables|Initialization|SetSelectionIndex _returnvalue_3))
          (Class|GeometryCollectionComponent|SetRestCollection (Variables|Default|GetGC_Plaster_Back) (Utilities|Array|Get(acopy) (Variables|Initialization|GetPlasterGeometry) _output_get_2)))))))

(fn InitializeStuds
  (bind _studgeometry (Variables|Initialization|GetStudGeometry))
  (bind _returnvalue (Utilities|Array|Length _studgeometry))
  (bind _returnvalue_2 (- _returnvalue 1))
  (bind _returnvalue_3 (Math|Random|RandomInteger _returnvalue_2))
  ;[1 1 1] Assign The First Stud With A Random GC From The Array
  (bind _output_get (Variables|Initialization|SetSelectionIndex (Math|Random|RandomInteger (- (Utilities|Array|Length (Variables|Initialization|GetStudGeometry)) 1))))
  (Class|GeometryCollectionComponent|SetRestCollection (Variables|Default|GetGC_Stud_1X29_1) (Utilities|Array|Get(acopy) (Variables|Initialization|GetStudGeometry) _output_get))
  ;[1 1 1] Select Another GC, But Do Not Use Previous One (FailSafe = Unless Only One Exist In Array)
  (Utilities|FlowControl|DoOnce false :!label _label
    (:Completed
      (if (and (!= _returnvalue 1) (== (Variables|Initialization|GetSelectionIndex) _returnvalue_3))
        (goto _label Reset)
        (else
          ;[1 1 1] Assign The Random GC To The Second Stud
          (bind _output_get_2 (Variables|Initialization|SetSelectionIndex _returnvalue_3))
          (Class|GeometryCollectionComponent|SetRestCollection (Variables|Default|GetGC_Stud_1X29_2) (Utilities|Array|Get(acopy) (Variables|Initialization|GetStudGeometry) _output_get_2)))))))

(fn SetAnchors
  (bind _gc_plaster_front (Variables|Default|GetGC_Plaster_Front))
  (bind _gc_stud_1x29_1 (Variables|Default|GetGC_Stud_1X29_1))
  (bind _gc_stud_1x29_2 (Variables|Default|GetGC_Stud_1X29_2))
  (bind _gc_plaster_back (Variables|Default|GetGC_Plaster_Back))
  (bind _initializationfields (Variables|/Script/GeometryCollectionEngine.GeometryCollectionComponent|GetInitializationFields _gc_plaster_back))
  (bind _initializationfields_2 (Variables|/Script/GeometryCollectionEngine.GeometryCollectionComponent|GetInitializationFields _gc_stud_1x29_2))
  (bind _initializationfields_3 (Variables|/Script/GeometryCollectionEngine.GeometryCollectionComponent|GetInitializationFields _gc_plaster_front))
  (bind _initializationfields_4 (Variables|/Script/GeometryCollectionEngine.GeometryCollectionComponent|GetInitializationFields _gc_stud_1x29_1))
  ;[1 1 1] Cast All Field Anchors (Log Bad Casts)
  (bind _asfs_anchor_field_custom (Utilities|Casting|CastToFS_AnchorField_Custom (Variables|/Script/Engine.ChildActorComponent|GetChildActor (Variables|Default|GetFS_AnchorField_Top)))
    (:then
      (bind _asfs_anchor_field_custom_2 (Utilities|Casting|CastToFS_AnchorField_Custom (Variables|/Script/Engine.ChildActorComponent|GetChildActor (Variables|Default|GetFS_AnchorField_Bottom)))
        (:then
          (bind _asfs_anchor_field_custom_3 (Utilities|Casting|CastToFS_AnchorField_Custom (Variables|/Script/Engine.ChildActorComponent|GetChildActor (Variables|Default|GetFS_AnchorField_Left)))
            (:then
              (bind _asfs_anchor_field_custom_4 (Utilities|Casting|CastToFS_AnchorField_Custom (Variables|/Script/Engine.ChildActorComponent|GetChildActor (Variables|Default|GetFS_AnchorField_Right)))
                (:then
                  ;[1 1 1] Assign Anchors To Plaster Sheets
                  (Utilities|Array|AddUnique _initializationfields_3 _asfs_anchor_field_custom)
                  (Utilities|Array|AddUnique _initializationfields_3 _asfs_anchor_field_custom_2)
                  (Utilities|Array|AddUnique _initializationfields_3 _asfs_anchor_field_custom_3)
                  (Utilities|Array|AddUnique _initializationfields_3 _asfs_anchor_field_custom_4)
                  (Utilities|Array|AddUnique _initializationfields _asfs_anchor_field_custom)
                  (Utilities|Array|AddUnique _initializationfields _asfs_anchor_field_custom_2)
                  (Utilities|Array|AddUnique _initializationfields _asfs_anchor_field_custom_3)
                  (Utilities|Array|AddUnique _initializationfields _asfs_anchor_field_custom_4)
                  ;[1 1 1] Assign Anchors To Studs
                  (Utilities|Array|AddUnique _initializationfields_4 _asfs_anchor_field_custom)
                  (Utilities|Array|AddUnique _initializationfields_4 _asfs_anchor_field_custom_2)
                  (Utilities|Array|AddUnique _initializationfields_2 _asfs_anchor_field_custom)
                  (Utilities|Array|AddUnique _initializationfields_2 _asfs_anchor_field_custom_2))
                (:CastFailed
                  (Class|AutomationBlueprintFunctionLibrary|AddExpectedLogError "Failed To Cast Anchors" :!label _label))))
            (:CastFailed
              (goto _label))))
        (:CastFailed
          (goto _label))))
    (:CastFailed
      (goto _label))))