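; Prefab plaster door frame built from Geometry Collection plaster sheets and studs, set up for Chaos destruction.
; The construction script assigns random rest collections from per-size arrays, with a reroll intended to avoid repeats within pairs.
; It then adds five child-actor anchor fields to the initialization fields of adjacent pieces, logging an error if any cast fails.
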(event EventBeginPlay
  (|CallParentFunction) ; This node is disabled and will not be called.\nDrag off pins to build functionality.
)

(event Collision|EventActorBeginOverlap
  (params (OtherActor :type Actor%20Object%20Reference))
  (|CallParentFunction OtherActor) ; This node is disabled and will not be called.\nDrag off pins to build functionality.
)

(event EventTick
  (params (DeltaSeconds :type Float%20%28single-precision%29))
  (|CallParentFunction DeltaSeconds) ; This node is disabled and will not be called.\nDrag off pins to build functionality.
)

(fn ConstructionScript
  (CallFunction|InitializePlasterSheets)
  (CallFunction|InitializeStuds)
  (CallFunction|SetAnchors))

(fn InitializePlasterSheets
  (bind _plastergeometrytop (Variables|Initialization|GetPlasterGeometryTop))
  (bind _plastergeometrybottom (Variables|Initialization|GetPlasterGeometryBottom))
  (bind _plastergeometrybottom_2 (Variables|Initialization|GetPlasterGeometryBottom))
  (bind _returnvalue (Utilities|Array|Length _plastergeometrybottom))
  (bind _returnvalue_2 (Utilities|Array|Length _plastergeometrytop))
  (bind _returnvalue_3 (Utilities|Array|Length _plastergeometrybottom_2))
  (bind _returnvalue_4 (- _returnvalue 1))
  (bind _returnvalue_5 (- _returnvalue_2 1))
  (bind _returnvalue_6 (- _returnvalue_3 1))
  (bind _returnvalue_7 (Math|Random|RandomInteger _returnvalue_4))
  (bind _returnvalue_8 (Math|Random|RandomInteger _returnvalue_6))
  (bind _returnvalue_9 (Math|Random|RandomInteger _returnvalue_5))
  ;[1 1 1] Initialize Top Plaster Sheets
  ;;[1 1 1] Assign A Random GC From The Array
  (bind _output_get (Variables|Initialization|SetSelectionIndex (Math|Random|RandomInteger (- (Utilities|Array|Length (Variables|Initialization|GetPlasterGeometryTop)) 1))))
  (Class|GeometryCollectionComponent|SetRestCollection (Variables|Default|GetGC_Plaster_Front_Top) (Utilities|Array|Get(acopy) (Variables|Initialization|GetPlasterGeometryTop) _output_get))
  ;;[1 1 1] Select Another GC, But Do Not Use Previous One (FailSafe = Unless Only One Exist In Array)
  (Utilities|FlowControl|DoOnce false :!label _label
    (:Completed
      (if (and (!= _returnvalue_2 1) (== (Variables|Initialization|GetSelectionIndex) _returnvalue_9))
        (goto _label Reset)
        (else
          ;;[1 1 1] Assign The Random GC
          (bind _output_get_2 (Variables|Initialization|SetSelectionIndex _returnvalue_9))
          (Class|GeometryCollectionComponent|SetRestCollection (Variables|Default|GetGC_Plaster_Back_Top) (Utilities|Array|Get(acopy) (Variables|Initialization|GetPlasterGeometryTop) _output_get_2))
          ;[1 1 1] Initialize Bottom Left Plaster Sheets
          ;;[1 1 1] Assign A Random GC From The Array
          (bind _output_get_3 (Variables|Initialization|SetSelectionIndex (Math|Random|RandomInteger (- (Utilities|Array|Length (Variables|Initialization|GetPlasterGeometryBottom)) 1))))
          (Class|GeometryCollectionComponent|SetRestCollection (Variables|Default|GetGC_Plaster_Front_Left) (Utilities|Array|Get(acopy) (Variables|Initialization|GetPlasterGeometryBottom) _output_get_3))
          ;;[1 1 1] Select Another GC, But Do Not Use Previous One (FailSafe = Unless Only One Exist In Array)
          (Utilities|FlowControl|DoOnce false :!label _label_2
            (:Completed
              (if (and (!= _returnvalue_3 1) (== (Variables|Initialization|GetSelectionIndex) _returnvalue_8))
                (goto _label_2 Reset)
                (else
                  ;;[1 1 1] Assign The Random GC
                  (bind _output_get_4 (Variables|Initialization|SetSelectionIndex _returnvalue_8))
                  (Class|GeometryCollectionComponent|SetRestCollection (Variables|Default|GetGC_Plaster_Back_Left) (Utilities|Array|Get(acopy) (Variables|Initialization|GetPlasterGeometryBottom) _output_get_4))
                  ;[1 1 1] Initialize Bottom Left Plaster Sheets
                  ;;[1 1 1] Assign A Random GC From The Array
                  (bind _output_get_5 (Variables|Initialization|SetSelectionIndex (Math|Random|RandomInteger (- (Utilities|Array|Length (Variables|Initialization|GetPlasterGeometryBottom)) 1))))
                  (Class|GeometryCollectionComponent|SetRestCollection (Variables|Default|GetGC_Plaster_Front_Right) (Utilities|Array|Get(acopy) (Variables|Initialization|GetPlasterGeometryBottom) _output_get_5))
                  ;;[1 1 1] Select Another GC, But Do Not Use Previous One (FailSafe = Unless Only One Exist In Array)
                  (Utilities|FlowControl|DoOnce false :!label _label_3
                    (:Completed
                      (if (and (!= _returnvalue 1) (== (Variables|Initialization|GetSelectionIndex) _returnvalue_7))
                        (goto _label_3 Reset)
                        (else
                          ;;[1 1 1] Assign The Random GC
                          (bind _output_get_6 (Variables|Initialization|SetSelectionIndex _returnvalue_7))
                          (Class|GeometryCollectionComponent|SetRestCollection (Variables|Default|GetGC_Plaster_Back_Right) (Utilities|Array|Get(acopy) (Variables|Initialization|GetPlasterGeometryBottom) _output_get_6)))))))))))))))

(fn InitializeStuds
  (bind _stud_1x195_geometry (Variables|Initialization|GetStud_1x195_Geometry))
  (bind _stud_1x09_geometry (Variables|Initialization|GetStud_1x09_Geometry))
  (bind _returnvalue (Utilities|Array|Length _stud_1x09_geometry))
  (bind _returnvalue_2 (Utilities|Array|Length _stud_1x195_geometry))
  (bind _returnvalue_3 (- _returnvalue 1))
  (bind _returnvalue_4 (- _returnvalue_2 1))
  (bind _returnvalue_5 (Math|Random|RandomInteger _returnvalue_3))
  (bind _returnvalue_6 (Math|Random|RandomInteger _returnvalue_4))
  ;[1 1 1] Assign The First Stud With A Random 1X29 GC From The Array
  (bind _output_get (Variables|Initialization|SetSelectionIndex (Math|Random|RandomInteger (- (Utilities|Array|Length (Variables|Initialization|GetStud_1x29_Geometry)) 1))))
  (Class|GeometryCollectionComponent|SetRestCollection (Variables|Default|GetGC_Stud_1X29_Horizontal) (Utilities|Array|Get(acopy) (Variables|Initialization|GetStud_1x29_Geometry) _output_get))
  ;[1 1 1] Initialize 1X195 Studs
  ;;[1 1 1] Assign  Random 1X195 Stud From Array
  (bind _output_get_2 (Variables|Initialization|SetSelectionIndex (Math|Random|RandomInteger (- (Utilities|Array|Length (Variables|Initialization|GetStud_1x195_Geometry)) 1))))
  (Class|GeometryCollectionComponent|SetRestCollection (Variables|Default|GetGC_Stud_1X195_Left) (Utilities|Array|Get(acopy) (Variables|Initialization|GetStud_1x195_Geometry) _output_get_2))
  ;;[1 1 1] Select Another GC, But Do Not Use Previous One (FailSafe = Unless Only One Exist In Array)
  (Utilities|FlowControl|DoOnce false :!label _label
    (:Completed
      (if (and (!= _returnvalue_2 1) (== (Variables|Initialization|GetSelectionIndex) _returnvalue_6))
        (goto _label Reset)
        (else
          ;;[1 1 1] Assign Different Random 1X195 Stud From Array
          (bind _output_get_3 (Variables|Initialization|SetSelectionIndex _returnvalue_6))
          (Class|GeometryCollectionComponent|SetRestCollection (Variables|Default|GetGC_Stud_1X195_Right) (Utilities|Array|Get(acopy) (Variables|Initialization|GetStud_1x195_Geometry) _output_get_3))
          ;[1 1 1] Initialize 1X09 Studs
          ;;[1 1 1] Assign  Random 1X09 Stud From Array
          (bind _output_get_4 (Variables|Initialization|SetSelectionIndex (Math|Random|RandomInteger (- (Utilities|Array|Length (Variables|Initialization|GetStud_1x09_Geometry)) 1))))
          (Class|GeometryCollectionComponent|SetRestCollection (Variables|Default|GetGC_Stud_1X09_Left) (Utilities|Array|Get(acopy) (Variables|Initialization|GetStud_1x09_Geometry) _output_get_4))
          ;;[1 1 1] Select Another GC, But Do Not Use Previous One (FailSafe = Unless Only One Exist In Array)
          (Utilities|FlowControl|DoOnce false :!label _label_2
            (:Completed
              (if (and (!= _returnvalue 1) (== (Variables|Initialization|GetSelectionIndex) _returnvalue_5))
                (goto _label_2 Reset)
                (else
                  ;;[1 1 1] Assign Different Random 1X09 Stud From Array
                  (bind _output_get_5 (Variables|Initialization|SetSelectionIndex _returnvalue_5))
                  (Class|GeometryCollectionComponent|SetRestCollection (Variables|Default|GetGC_Stud_1X09_Right) (Utilities|Array|Get(acopy) (Variables|Initialization|GetStud_1x09_Geometry) _output_get_5)))))))))))

(fn SetAnchors
  (bind _gc_plaster_back_right (Variables|Default|GetGC_Plaster_Back_Right))
  (bind _gc_plaster_front_right (Variables|Default|GetGC_Plaster_Front_Right))
  (bind _gc_plaster_front_left (Variables|Default|GetGC_Plaster_Front_Left))
  (bind _gc_plaster_back_left (Variables|Default|GetGC_Plaster_Back_Left))
  (bind _gc_stud_1x29_horizontal (Variables|Default|GetGC_Stud_1X29_Horizontal))
  (bind _gc_plaster_front_top (Variables|Default|GetGC_Plaster_Front_Top))
  (bind _gc_plaster_back_top (Variables|Default|GetGC_Plaster_Back_Top))
  (bind _initializationfields (Variables|/Script/GeometryCollectionEngine.GeometryCollectionComponent|GetInitializationFields _gc_plaster_front_top))
  (bind _initializationfields_2 (Variables|/Script/GeometryCollectionEngine.GeometryCollectionComponent|GetInitializationFields _gc_plaster_back_top))
  (bind _initializationfields_3 (Variables|/Script/GeometryCollectionEngine.GeometryCollectionComponent|GetInitializationFields _gc_plaster_back_right))
  (bind _initializationfields_4 (Variables|/Script/GeometryCollectionEngine.GeometryCollectionComponent|GetInitializationFields _gc_plaster_front_right))
  (bind _initializationfields_5 (Variables|/Script/GeometryCollectionEngine.GeometryCollectionComponent|GetInitializationFields _gc_plaster_front_left))
  (bind _initializationfields_6 (Variables|/Script/GeometryCollectionEngine.GeometryCollectionComponent|GetInitializationFields _gc_plaster_back_left))
  (bind _initializationfields_7 (Variables|/Script/GeometryCollectionEngine.GeometryCollectionComponent|GetInitializationFields _gc_stud_1x29_horizontal))
  ;[1 1 1] Cast All Field Anchors (Log Bad Casts)
  (bind _asfs_anchor_field_custom (Utilities|Casting|CastToFS_AnchorField_Custom (Variables|/Script/Engine.ChildActorComponent|GetChildActor (Variables|Default|GetFS_AnchorField_Top)))
    (:then
      (bind _asfs_anchor_field_custom_2 (Utilities|Casting|CastToFS_AnchorField_Custom (Variables|/Script/Engine.ChildActorComponent|GetChildActor (Variables|Default|GetFS_AnchorField_Bottom_Left)))
        (:then
          (bind _asfs_anchor_field_custom_3 (Utilities|Casting|CastToFS_AnchorField_Custom (Variables|/Script/Engine.ChildActorComponent|GetChildActor (Variables|Default|GetFS_AnchorField_Bottom_Right)))
            (:then
              (bind _asfs_anchor_field_custom_4 (Utilities|Casting|CastToFS_AnchorField_Custom (Variables|/Script/Engine.ChildActorComponent|GetChildActor (Variables|Default|GetFS_AnchorField_Left)))
                (:then
                  (bind _asfs_anchor_field_custom_5 (Utilities|Casting|CastToFS_AnchorField_Custom (Variables|/Script/Engine.ChildActorComponent|GetChildActor (Variables|Default|GetFS_AnchorField_Right)))
                    (:then
                      ;[1 1 1] Assign Anchors To Top Plaster Sheets
                      (Utilities|Array|AddUnique _initializationfields _asfs_anchor_field_custom)
                      (Utilities|Array|AddUnique _initializationfields _asfs_anchor_field_custom_4)
                      (Utilities|Array|AddUnique _initializationfields _asfs_anchor_field_custom_5)
                      (Utilities|Array|AddUnique _initializationfields_2 _asfs_anchor_field_custom)
                      (Utilities|Array|AddUnique _initializationfields_2 _asfs_anchor_field_custom_4)
                      (Utilities|Array|AddUnique _initializationfields_2 _asfs_anchor_field_custom_5)
                      ;[1 1 1] Assign Anchors To Left Plaster Sheets
                      (Utilities|Array|AddUnique _initializationfields_5 _asfs_anchor_field_custom_2)
                      (Utilities|Array|AddUnique _initializationfields_5 _asfs_anchor_field_custom_4)
                      (Utilities|Array|AddUnique _initializationfields_6 _asfs_anchor_field_custom_2)
                      (Utilities|Array|AddUnique _initializationfields_6 _asfs_anchor_field_custom_4)
                      ;[1 1 1] Assign Anchors To Right Plaster Sheets
                      (Utilities|Array|AddUnique _initializationfields_4 _asfs_anchor_field_custom_3)
                      (Utilities|Array|AddUnique _initializationfields_4 _asfs_anchor_field_custom_5)
                      (Utilities|Array|AddUnique _initializationfields_3 _asfs_anchor_field_custom_3)
                      (Utilities|Array|AddUnique _initializationfields_3 _asfs_anchor_field_custom_5)
                      ;[1 1 1] Assign Anchors To 1X29 Horisontal Stud
                      (Utilities|Array|AddUnique _initializationfields_7 _asfs_anchor_field_custom_4)
                      (Utilities|Array|AddUnique _initializationfields_7 _asfs_anchor_field_custom_5)
                      ;[1 1 1] Assign Anchors To 1X09 Vertical Studs
                      (Utilities|Array|AddUnique (Variables|/Script/GeometryCollectionEngine.GeometryCollectionComponent|GetInitializationFields (Variables|Default|GetGC_Stud_1X09_Left)) _asfs_anchor_field_custom)
                      (Utilities|Array|AddUnique (Variables|/Script/GeometryCollectionEngine.GeometryCollectionComponent|GetInitializationFields (Variables|Default|GetGC_Stud_1X09_Right)) _asfs_anchor_field_custom)
                      ;[1 1 1] Assign Anchors To 1X195 Vertical Studs
                      (Utilities|Array|AddUnique (Variables|/Script/GeometryCollectionEngine.GeometryCollectionComponent|GetInitializationFields (Variables|Default|GetGC_Stud_1X195_Left)) _asfs_anchor_field_custom_2)
                      (Utilities|Array|AddUnique (Variables|/Script/GeometryCollectionEngine.GeometryCollectionComponent|GetInitializationFields (Variables|Default|GetGC_Stud_1X195_Right)) _asfs_anchor_field_custom_3))
                    (:CastFailed
                      (Class|AutomationBlueprintFunctionLibrary|AddExpectedLogError "Failed To Cast Anchors" :!label _label))))
                (:CastFailed
                  (goto _label))))
            (:CastFailed
              (goto _label))))
        (:CastFailed
          (goto _label))))
    (:CastFailed
      (goto _label))))