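; Destructible 3x3 concrete wall prefab tile, built around a Chaos Geometry Collection.
; The construction script assigns a random rest collection from the ConcreteGeometry array, though its Length - 1 random bound never selects the last entry.
; It then adds the top child-actor anchor field to the wall's initialization fields, calling AddExpectedLogError if the cast fails.
; The event graph holds only disabled stubs.
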(event EventBeginPlay
  (|CallParentFunction) ; This node is disabled and will not be called.\nDrag off pins to build functionality.
)

(event Collision|EventActorBeginOverlap
  (params (OtherActor :type Actor%20Object%20Reference))
  (|CallParentFunction OtherActor) ; This node is disabled and will not be called.\nDrag off pins to build functionality.
)

(event EventTick
  (params (DeltaSeconds :type Float%20%28single-precision%29))
  (|CallParentFunction DeltaSeconds) ; This node is disabled and will not be called.\nDrag off pins to build functionality.
)

(fn ConstructionScript
  (CallFunction|InitializeConcreteWall)
  (CallFunction|SetAnchors))

(fn InitializeConcreteWall
  ;[1 1 1] Assign The Front Plaster Sheet With A Random GC From The Array
  (bind _output_get (Variables|Initialization|SetSelectionIndex (Math|Random|RandomInteger (- (Utilities|Array|Length (Variables|Initialization|GetConcreteGeometry)) 1))))
  (Class|GeometryCollectionComponent|SetRestCollection (Variables|Default|GetGC_ConcreteWall) (Utilities|Array|Get(acopy) (Variables|Initialization|GetConcreteGeometry) _output_get)))

(fn SetAnchors
  ;[1 1 1] Cast Field Anchor (Log Bad Casts), And Assign To Concrete Wall
  (bind _asfs_anchor_field_custom (Utilities|Casting|CastToFS_AnchorField_Custom (Variables|/Script/Engine.ChildActorComponent|GetChildActor (Variables|Default|GetFS_AnchorField_Top)))
    (:then
      (Utilities|Array|AddUnique (Variables|/Script/GeometryCollectionEngine.GeometryCollectionComponent|GetInitializationFields (Variables|Default|GetGC_ConcreteWall)) _asfs_anchor_field_custom))
    (:CastFailed
      (Class|AutomationBlueprintFunctionLibrary|AddExpectedLogError "Failed To Cast Anchors"))))